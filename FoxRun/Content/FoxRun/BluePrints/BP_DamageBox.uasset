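; BP_DamageBox is a damage volume for the FoxRun game that reduces player health when its Box component is overlapped.
; Any overlap, with no check on the other actor, subtracts HealthDamage from Health on GM_MainGameInstance and prints the result.
; If Health is still zero or above, it destroys the player's fox character after a short delay; below zero, it opens the FR_Loss level.
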(event OnComponentBeginOverlap(Box)
  (params (OverlappedComponent :type Primitive%20Component%20Object%20Reference) (OtherActor :type Actor%20Object%20Reference) (OtherComp :type Primitive%20Component%20Object%20Reference) (OtherBodyIndex :type Integer) (bFromSweep :type Boolean) (SweepResult :type Hit%20Result%20Structure%20%28by%20ref%29))
  (bind _asgm_main_game_instance (Utilities|Casting|CastToGM_MainGameInstance (Game|GetGameInstance)))
  (bind _output_get (Variables|/Game/FoxRun/BluePrints/GM_MainGameInstance.GM_MainGameInstance_C|Sethealth _asgm_main_game_instance (- (Variables|/Game/FoxRun/BluePrints/GM_MainGameInstance.GM_MainGameInstance_C|Gethealth _asgm_main_game_instance) (Variables|Default|GetHealth%20Damage))))
  (Development|PrintString (Utilities|String|ToString(Float) _output_get))
  (if (<= 0.0 _output_get)
    (bind _asbp_fox_player (Utilities|Casting|CastToBP_fox_PLayer (Game|GetPlayerCharacter 0)))
    (Utilities|FlowControl|Delay 0.2)
    (Actor|DestroyActor _asbp_fox_player)
    (else
      (Game|OpenLevel(byName) "FR_Loss"))))

(event EventBeginPlay)

(event EventTick
  (params (DeltaSeconds :type Float%20%28single-precision%29)))

(fn ConstructionScript)