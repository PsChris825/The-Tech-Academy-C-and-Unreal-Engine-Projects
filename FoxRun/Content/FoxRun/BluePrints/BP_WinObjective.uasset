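; BP_WinObjective is the win trigger for FoxRun, ending the run when its Box component is overlapped.
; On overlap it copies the minutes and seconds from the GM_FR game mode into GM_MainGameInstance as LastMinute and LastSecond, then opens the FR_Win level.
; The overlapping actor is not checked, so any overlap the Box registers triggers the win.
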(event OnComponentBeginOverlap(Box)
  (params (OverlappedComponent :type Primitive%20Component%20Object%20Reference) (OtherActor :type Actor%20Object%20Reference) (OtherComp :type Primitive%20Component%20Object%20Reference) (OtherBodyIndex :type Integer) (bFromSweep :type Boolean) (SweepResult :type Hit%20Result%20Structure%20%28by%20ref%29))
  (bind _asgm_fr (Utilities|Casting|CastToGM_FR (Game|GetGameMode)))
  (bind _asgm_main_game_instance (Utilities|Casting|CastToGM_MainGameInstance (Game|GetGameInstance)))
  (Variables|/Game/FoxRun/BluePrints/GM_MainGameInstance.GM_MainGameInstance_C|SetLastMinute _asgm_main_game_instance (Math|Conversions|ToFloat(Integer) (Variables|/Game/FoxRun/BluePrints/GM_FR.GM_FR_C|GetMinutes _asgm_fr)))
  (bind _output_get (Variables|/Game/FoxRun/BluePrints/GM_MainGameInstance.GM_MainGameInstance_C|SetLastSecond _asgm_main_game_instance (Math|Conversions|ToFloat(Integer) (Variables|/Game/FoxRun/BluePrints/GM_FR.GM_FR_C|GetSeconds _asgm_fr))))
  (Game|OpenLevel(byName) "FR_Win"))

(event EventBeginPlay)

(event EventTick
  (params (DeltaSeconds :type Float%20%28single-precision%29)))

(fn ConstructionScript)